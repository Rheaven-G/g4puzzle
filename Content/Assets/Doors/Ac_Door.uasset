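; Key-locked door actor that swings open when something enters its trigger box after the key has been found.
; On BeginPlay it binds to the KeyFound event of a referenced KeyActor, which sets a HasKey flag.
; Box overlap plays a timeline that lerps the hinge's yaw, and ending overlap reverses it to close the door.
; The overlap events do not filter which actor triggers them.
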(event OnComponentBeginOverlap(Box)
  (params (OverlappedComponent :type Primitive%20Component%20Object%20Reference) (OtherActor :type Actor%20Object%20Reference) (OtherComp :type Primitive%20Component%20Object%20Reference) (OtherBodyIndex :type Integer) (bFromSweep :type Boolean) (SweepResult :type Hit%20Result%20Structure%20%28by%20ref%29))
  (if (Variables|Default|GetHasKey)
    (CallFunction|OpenDoor)))

(event OnComponentEndOverlap(Box)
  (params (OverlappedComponent :type Primitive%20Component%20Object%20Reference) (OtherActor :type Actor%20Object%20Reference) (OtherComp :type Primitive%20Component%20Object%20Reference) (OtherBodyIndex :type Integer))
  (CallFunction|CloseDoor))

(event Custom|OpenDoor
  (bind _open_door (Timeline|Timeline_Door Play)
    (:Update
      (Transformation|SetRelativeRotation (Variables|Default|GetDoor_Hinge) (Math|Rotator|MakeRotator 0.0 0.0 (Math|Float|Lerp 0.0 1.3e+02 _open_door)) false false))))

(event Custom|CloseDoor
  (bind _open_door (Timeline|Timeline_Door Reverse)
    (:Update
      (Transformation|SetRelativeRotation (Variables|Default|GetDoor_Hinge) (Math|Rotator|MakeRotator 0.0 0.0 (Math|Float|Lerp 0.0 1.3e+02 _open_door)) false false))))

(event Custom|KeyFound
  (Variables|Default|SetHasKey true))

(event EventBeginPlay
  (EventDispatchers|BindEventtoKeyFound (Variables|Default|GetKeyActor) (delegate Custom|KeyFound)))

(event Collision|EventActorBeginOverlap
  (params (OtherActor :type Actor%20Object%20Reference)))

(event EventTick
  (params (DeltaSeconds :type Float%20%28single-precision%29)))

(fn ConstructionScript)